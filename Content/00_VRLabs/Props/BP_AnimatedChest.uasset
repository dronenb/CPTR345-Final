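; BP_AnimatedChest is a VR Labs chest prop whose lid animates open and closed.
; OpenChest plays ChestTimeline and CloseChest reverses it, each printing a debug message, while the Turnon and TurnOff events simply forward to them.
; Each timeline update passes the LidMovement track through a sine, then scales and offsets it to set the Lid's relative pitch.
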(event Custom|OpenChest
  (Development|PrintString "Opening Chest...")
  (bind _lidmovement (Timeline|ChestTimeline Play)
    (:Update
      (Transformation|SetRelativeRotation (Variables|Default|GetLid) (Math|Rotator|MakeRotator 0.0 (- (* (Math|Trig|Sin(Radians) _lidmovement) -45.0) 45.0) 0.0) false false))))

(event Custom|CloseChest
  (Development|PrintString "Closing Chest...")
  (bind _lidmovement (Timeline|ChestTimeline Reverse)
    (:Update
      (Transformation|SetRelativeRotation (Variables|Default|GetLid) (Math|Rotator|MakeRotator 0.0 (- (* (Math|Trig|Sin(Radians) _lidmovement) -45.0) 45.0) 0.0) false false))))

(event EventBeginPlay)

(event Collision|EventActorBeginOverlap
  (params (OtherActor :type Actor%20Object%20Reference)))

(event EventTick
  (params (DeltaSeconds :type Float%20%28single-precision%29)))

(event EventTurnOff
  (CallFunction|CloseChest))

(event EventTurnon
  (CallFunction|OpenChest))

(fn ConstructionScript)
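; VR piano prop with twelve keys that doubles as a note-sequence puzzle.
; Key overlaps play per-key timelines that offset keys along their down vector, and end overlaps reverse them.
; Timeline Finished events play that key's sound and check it against Sequence, resetting progress on a wrong note.
; Completing the sequence plays a Mario sound cue and calls TurnOn on Target.
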(event OnComponentBeginOverlap(C)
  (params (OverlappedComponent :type Primitive%20Component%20Object%20Reference) (OtherActor :type Actor%20Object%20Reference) (OtherComp :type Primitive%20Component%20Object%20Reference) (OtherBodyIndex :type Integer) (bFromSweep :type Boolean) (SweepResult :type Hit%20Result%20Structure%20%28by%20ref%29))
  (bind _cpercenttravel (Timeline|C%20Animation Play)
    (:Update
      (CallFunction|ComputeLocation 0 _cpercenttravel))
    (:Finished
      (CallFunction|PlaySound))))

(event OnComponentEndOverlap(C)
  (params (OverlappedComponent :type Primitive%20Component%20Object%20Reference) (OtherActor :type Actor%20Object%20Reference) (OtherComp :type Primitive%20Component%20Object%20Reference) (OtherBodyIndex :type Integer))
  (bind _cpercenttravel (Timeline|C%20Animation Reverse)
    (:Update
      (CallFunction|ComputeLocation 0 _cpercenttravel))
    (:Finished
      (CallFunction|PlaySound))))

(event OnComponentBeginOverlap(D#)
  (params (OverlappedComponent :type Primitive%20Component%20Object%20Reference) (OtherActor :type Actor%20Object%20Reference) (OtherComp :type Primitive%20Component%20Object%20Reference) (OtherBodyIndex :type Integer) (bFromSweep :type Boolean) (SweepResult :type Hit%20Result%20Structure%20%28by%20ref%29))
  (bind _percenttravel (Timeline|D#%20Animation Play)
    (:Update
      (CallFunction|ComputeLocation 3 _percenttravel))
    (:Finished
      (CallFunction|PlaySound 3))))

(event OnComponentEndOverlap(D#)
  (params (OverlappedComponent :type Primitive%20Component%20Object%20Reference) (OtherActor :type Actor%20Object%20Reference) (OtherComp :type Primitive%20Component%20Object%20Reference) (OtherBodyIndex :type Integer))
  (bind _percenttravel (Timeline|D#%20Animation Reverse)
    (:Update
      (CallFunction|ComputeLocation 3 _percenttravel))
    (:Finished
      (CallFunction|PlaySound 3))))

(event OnComponentBeginOverlap(E)
  (params (OverlappedComponent :type Primitive%20Component%20Object%20Reference) (OtherActor :type Actor%20Object%20Reference) (OtherComp :type Primitive%20Component%20Object%20Reference) (OtherBodyIndex :type Integer) (bFromSweep :type Boolean) (SweepResult :type Hit%20Result%20Structure%20%28by%20ref%29))
  (bind _percenttravel (Timeline|E%20Animation Play)
    (:Update
      (CallFunction|ComputeLocation 4 _percenttravel))
    (:Finished
      (CallFunction|PlaySound 4))))

(event OnComponentEndOverlap(E)
  (params (OverlappedComponent :type Primitive%20Component%20Object%20Reference) (OtherActor :type Actor%20Object%20Reference) (OtherComp :type Primitive%20Component%20Object%20Reference) (OtherBodyIndex :type Integer))
  (bind _percenttravel (Timeline|E%20Animation Reverse)
    (:Update
      (CallFunction|ComputeLocation 4 _percenttravel))
    (:Finished
      (CallFunction|PlaySound 4))))

(event OnComponentBeginOverlap(F)
  (params (OverlappedComponent :type Primitive%20Component%20Object%20Reference) (OtherActor :type Actor%20Object%20Reference) (OtherComp :type Primitive%20Component%20Object%20Reference) (OtherBodyIndex :type Integer) (bFromSweep :type Boolean) (SweepResult :type Hit%20Result%20Structure%20%28by%20ref%29))
  (bind _percenttravel (Timeline|F%20Animation Play)
    (:Update
      (CallFunction|ComputeLocation 5 _percenttravel))
    (:Finished
      (CallFunction|PlaySound 5))))

(event OnComponentEndOverlap(F)
  (params (OverlappedComponent :type Primitive%20Component%20Object%20Reference) (OtherActor :type Actor%20Object%20Reference) (OtherComp :type Primitive%20Component%20Object%20Reference) (OtherBodyIndex :type Integer))
  (bind _percenttravel (Timeline|F%20Animation Reverse)
    (:Update
      (CallFunction|ComputeLocation 5 _percenttravel))
    (:Finished
      (CallFunction|PlaySound 5))))

(event OnComponentBeginOverlap(F#)
  (params (OverlappedComponent :type Primitive%20Component%20Object%20Reference) (OtherActor :type Actor%20Object%20Reference) (OtherComp :type Primitive%20Component%20Object%20Reference) (OtherBodyIndex :type Integer) (bFromSweep :type Boolean) (SweepResult :type Hit%20Result%20Structure%20%28by%20ref%29))
  (bind _percenttravel (Timeline|F#%20Animation Play)
    (:Update
      (CallFunction|ComputeLocation 6 _percenttravel))
    (:Finished
      (CallFunction|PlaySound 6))))

(event OnComponentEndOverlap(F#)
  (params (OverlappedComponent :type Primitive%20Component%20Object%20Reference) (OtherActor :type Actor%20Object%20Reference) (OtherComp :type Primitive%20Component%20Object%20Reference) (OtherBodyIndex :type Integer))
  (bind _percenttravel (Timeline|F#%20Animation Reverse)
    (:Update
      (CallFunction|ComputeLocation 6 _percenttravel))
    (:Finished
      (CallFunction|PlaySound 6))))

(event OnComponentBeginOverlap(G)
  (params (OverlappedComponent :type Primitive%20Component%20Object%20Reference) (OtherActor :type Actor%20Object%20Reference) (OtherComp :type Primitive%20Component%20Object%20Reference) (OtherBodyIndex :type Integer) (bFromSweep :type Boolean) (SweepResult :type Hit%20Result%20Structure%20%28by%20ref%29))
  (bind _percenttravel (Timeline|G%20Animation Play)
    (:Update
      (CallFunction|ComputeLocation 7 _percenttravel))
    (:Finished
      (CallFunction|PlaySound 7))))

(event OnComponentEndOverlap(G)
  (params (OverlappedComponent :type Primitive%20Component%20Object%20Reference) (OtherActor :type Actor%20Object%20Reference) (OtherComp :type Primitive%20Component%20Object%20Reference) (OtherBodyIndex :type Integer))
  (bind _percenttravel (Timeline|G%20Animation Reverse)
    (:Update
      (CallFunction|ComputeLocation 7 _percenttravel))
    (:Finished
      (CallFunction|PlaySound 7))))

(event OnComponentBeginOverlap(G#)
  (params (OverlappedComponent :type Primitive%20Component%20Object%20Reference) (OtherActor :type Actor%20Object%20Reference) (OtherComp :type Primitive%20Component%20Object%20Reference) (OtherBodyIndex :type Integer) (bFromSweep :type Boolean) (SweepResult :type Hit%20Result%20Structure%20%28by%20ref%29))
  (bind _percenttravel (Timeline|G#%20Animation Play)
    (:Update
      (CallFunction|ComputeLocation 8 _percenttravel))
    (:Finished
      (CallFunction|PlaySound 8))))

(event OnComponentEndOverlap(G#)
  (params (OverlappedComponent :type Primitive%20Component%20Object%20Reference) (OtherActor :type Actor%20Object%20Reference) (OtherComp :type Primitive%20Component%20Object%20Reference) (OtherBodyIndex :type Integer))
  (bind _percenttravel (Timeline|G#%20Animation Reverse)
    (:Update
      (CallFunction|ComputeLocation 8 _percenttravel))
    (:Finished
      (CallFunction|PlaySound 8))))

(event OnComponentBeginOverlap(C#)
  (params (OverlappedComponent :type Primitive%20Component%20Object%20Reference) (OtherActor :type Actor%20Object%20Reference) (OtherComp :type Primitive%20Component%20Object%20Reference) (OtherBodyIndex :type Integer) (bFromSweep :type Boolean) (SweepResult :type Hit%20Result%20Structure%20%28by%20ref%29))
  (bind _percenttravel (Timeline|C#%20Animation Play)
    (:Update
      (CallFunction|ComputeLocation 1 _percenttravel))
    (:Finished
      (CallFunction|PlaySound 1))))

(event OnComponentBeginOverlap(A)
  (params (OverlappedComponent :type Primitive%20Component%20Object%20Reference) (OtherActor :type Actor%20Object%20Reference) (OtherComp :type Primitive%20Component%20Object%20Reference) (OtherBodyIndex :type Integer) (bFromSweep :type Boolean) (SweepResult :type Hit%20Result%20Structure%20%28by%20ref%29))
  (bind _percenttravel (Timeline|A%20Animation Play)
    (:Update
      (CallFunction|ComputeLocation 9 _percenttravel))
    (:Finished
      (CallFunction|PlaySound 9))))

(event OnComponentEndOverlap(A)
  (params (OverlappedComponent :type Primitive%20Component%20Object%20Reference) (OtherActor :type Actor%20Object%20Reference) (OtherComp :type Primitive%20Component%20Object%20Reference) (OtherBodyIndex :type Integer))
  (bind _percenttravel (Timeline|A%20Animation Reverse)
    (:Update
      (CallFunction|ComputeLocation 9 _percenttravel))
    (:Finished
      (CallFunction|PlaySound 9))))

(event OnComponentEndOverlap(C#)
  (params (OverlappedComponent :type Primitive%20Component%20Object%20Reference) (OtherActor :type Actor%20Object%20Reference) (OtherComp :type Primitive%20Component%20Object%20Reference) (OtherBodyIndex :type Integer))
  (bind _percenttravel (Timeline|C#%20Animation Reverse)
    (:Update
      (CallFunction|ComputeLocation 1 _percenttravel))
    (:Finished
      (CallFunction|PlaySound 1))))

(event OnComponentBeginOverlap(A#)
  (params (OverlappedComponent :type Primitive%20Component%20Object%20Reference) (OtherActor :type Actor%20Object%20Reference) (OtherComp :type Primitive%20Component%20Object%20Reference) (OtherBodyIndex :type Integer) (bFromSweep :type Boolean) (SweepResult :type Hit%20Result%20Structure%20%28by%20ref%29))
  (bind _percenttravel (Timeline|A#%20Animation Play)
    (:Update
      (CallFunction|ComputeLocation 10 _percenttravel))
    (:Finished
      (CallFunction|PlaySound 10))))

(event OnComponentEndOverlap(A#)
  (params (OverlappedComponent :type Primitive%20Component%20Object%20Reference) (OtherActor :type Actor%20Object%20Reference) (OtherComp :type Primitive%20Component%20Object%20Reference) (OtherBodyIndex :type Integer))
  (bind _percenttravel (Timeline|A#%20Animation Reverse)
    (:Update
      (CallFunction|ComputeLocation 10 _percenttravel))
    (:Finished
      (CallFunction|PlaySound 10))))

(event OnComponentBeginOverlap(B)
  (params (OverlappedComponent :type Primitive%20Component%20Object%20Reference) (OtherActor :type Actor%20Object%20Reference) (OtherComp :type Primitive%20Component%20Object%20Reference) (OtherBodyIndex :type Integer) (bFromSweep :type Boolean) (SweepResult :type Hit%20Result%20Structure%20%28by%20ref%29))
  (bind _percenttravel (Timeline|B%20Animation Play)
    (:Update
      (CallFunction|ComputeLocation 11 _percenttravel))
    (:Finished
      (CallFunction|PlaySound 11))))

(event OnComponentEndOverlap(B)
  (params (OverlappedComponent :type Primitive%20Component%20Object%20Reference) (OtherActor :type Actor%20Object%20Reference) (OtherComp :type Primitive%20Component%20Object%20Reference) (OtherBodyIndex :type Integer))
  (bind _percenttravel (Timeline|B%20Animation Reverse)
    (:Update
      (CallFunction|ComputeLocation 11 _percenttravel))
    (:Finished
      (CallFunction|PlaySound 11))))

(event OnComponentBeginOverlap(D)
  (params (OverlappedComponent :type Primitive%20Component%20Object%20Reference) (OtherActor :type Actor%20Object%20Reference) (OtherComp :type Primitive%20Component%20Object%20Reference) (OtherBodyIndex :type Integer) (bFromSweep :type Boolean) (SweepResult :type Hit%20Result%20Structure%20%28by%20ref%29))
  (bind _percenttravel (Timeline|D%20Animation Play)
    (:Update
      (CallFunction|ComputeLocation 2 _percenttravel))
    (:Finished
      (CallFunction|PlaySound 2))))

(event OnComponentEndOverlap(D)
  (params (OverlappedComponent :type Primitive%20Component%20Object%20Reference) (OtherActor :type Actor%20Object%20Reference) (OtherComp :type Primitive%20Component%20Object%20Reference) (OtherBodyIndex :type Integer))
  (bind _percenttravel (Timeline|D%20Animation Reverse)
    (:Update
      (CallFunction|ComputeLocation 2 _percenttravel))
    (:Finished
      (CallFunction|PlaySound 2))))

(event EventBeginPlay
  (bind _output_get (Variables|Default|SetKeysArray (Utilities|Array|MakeArray (Variables|Default|GetC) (Variables|Default|GetC#) (Variables|Default|GetD) (Variables|Default|GetD#) (Variables|Default|GetE) (Variables|Default|GetF) (Variables|Default|GetF#) (Variables|Default|GetG) (Variables|Default|GetG#) (Variables|Default|GetA) (Variables|Default|GetA#) (Variables|Default|GetB))))
  (for _array_element _output_get
    (Utilities|Array|AppendArray (Variables|Default|GetInitialLocations) (Utilities|Array|MakeArray (Transformation|GetWorldLocation _array_element)))
    (Utilities|Array|AppendArray (Variables|Default|GetCurrentLocations) (Utilities|Array|MakeArray (Transformation|GetWorldLocation _array_element))))
  (bind _output_get_2 (Variables|Default|SetTimelines (Utilities|Array|MakeArray (Variables|Default|GetC%20Animation) (Variables|Default|GetC#%20Animation) (Variables|Default|GetD%20Animation) (Variables|Default|GetD#%20Animation) (Variables|Default|GetE%20Animation) (Variables|Default|GetF%20Animation) (Variables|Default|GetF#%20Animation) (Variables|Default|GetG%20Animation) (Variables|Default|GetG#%20Animation) (Variables|Default|GetA%20Animation) (Variables|Default|GetA#%20Animation) (Variables|Default|GetB%20Animation))))
  (for _array_element_2 _output_get_2
    (Components|Timeline|SetPlayRate _array_element_2 (Variables|Default|GetAnimationPlayRate))))

(event Collision|EventActorBeginOverlap
  (params (OtherActor :type Actor%20Object%20Reference)))

(event EventTick
  (params (DeltaSeconds :type Float%20%28single-precision%29)))

(fn ConstructionScript)

(fn ComputeLocation
  (params (Index :type Integer) (PercentTravel :type Float%20%28single-precision%29))
  (bind _keysarray (Variables|Default|GetKeysArray))
  (bind _maximumtravel (Variables|Default|GetMaximumTravel))
  (bind _initiallocations (Variables|Default|GetInitialLocations))
  (bind _returnvalue (* PercentTravel _maximumtravel))
  (bind _output (Utilities|Array|Get(acopy) _keysarray Index))
  (bind _output_2 (Utilities|Array|Get(acopy) _initiallocations Index))
  (bind _returnvalue_2 (Math|Vector|GetUpVector _output))
  (bind _returnvalue_3 (* _returnvalue_2 _returnvalue))
  (bind _returnvalue_4 (- _output_2 _returnvalue_3))
  (Utilities|Array|SetArrayElem (Variables|Default|GetCurrentLocations) Index _returnvalue_4)
  (Transformation|SetWorldLocation _output _returnvalue_4 false false))

(fn PlaySound
  (params (Index :type Integer))
  (Audio|PlaySoundatLocation (Utilities|Array|Get(acopy) (Variables|Default|GetKeySounds) Index) (Utilities|Array|Get(acopy) (Variables|Default|GetCurrentLocations) Index) "0, 0, 0" 1.0 1.0 0.0 0 0 0)
  (CallFunction|CheckSequence Index))

(fn CheckSequence
  (params (Input :type Integer))
  (if (== (Utilities|Array|Get(acopy) (Variables|Default|GetSequence) (Variables|Default|GetCurrentSequenceStep)) Input)
    (bind _output_get (Variables|Default|SetCurrentSequenceStep (+ (Variables|Default|GetCurrentSequenceStep) 1)))
    (if (== (Utilities|Array|Length (Variables|Default|GetSequence)) _output_get)
      (Audio|PlaySoundatLocation "/Game/00_VRLabs/Props/Sounds/mariosound_Cue.mariosound_Cue" (Utilities|Array|Get(acopy) (Variables|Default|GetCurrentLocations) Input) "0, 0, 0" 1.0 1.0 0.0 0 0 0)
      (Default|Turnon (Variables|Default|GetTarget)))
    (else
      (Variables|Default|SetCurrentSequenceStep 0))))
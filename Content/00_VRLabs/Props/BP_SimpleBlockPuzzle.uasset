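; BP_SimpleBlockPuzzle is a VR puzzle prop solved by placing a red and a blue block in their matching locations.
; Overlapping the correct block with its location releases it from the grab component and snaps it on.
; Dropping a block toggles its physics by overlap and updates its placed flag.
; Both flags drive the red/green solved light, but only overlap events switch the Target on or off.
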(event OnComponentBeginOverlap(BlueCubeLocation)
  (params (OverlappedComponent :type Primitive%20Component%20Object%20Reference) (OtherActor :type Actor%20Object%20Reference) (OtherComp :type Primitive%20Component%20Object%20Reference) (OtherBodyIndex :type Integer) (bFromSweep :type Boolean) (SweepResult :type Hit%20Result%20Structure%20%28by%20ref%29))
  (bind _target (Variables|Default|GetTarget))
  (bind _blockmatches (CallFunction|TrytoAttachBlock OverlappedComponent OtherComp (Variables|Default|GetBlueBlock) (Variables|Default|GetBlueBlockGrabComponent)))
  (Variables|Default|SetIsBlueBlockInPlace _blockmatches)
  (bind _solved (CallFunction|CheckforSolvedPuzzle))
  (if _solved
    (Default|Turnon _target)
    (else
      (Default|TurnOff _target)
      (Development|PrintString "Turned off"))))

(event OnDropped(RedBlockGrabComponent)
  (bind _isoverlapping (CallFunction|SetPhysicsonRelease (Variables|Default|GetRedBlock) (Variables|Default|GetRedCubeLocation)))
  (Variables|Default|SetIsRedBlockInPlace _isoverlapping)
  (CallFunction|CheckforSolvedPuzzle))

(event OnComponentBeginOverlap(RedCubeLocation)
  (params (OverlappedComponent :type Primitive%20Component%20Object%20Reference) (OtherActor :type Actor%20Object%20Reference) (OtherComp :type Primitive%20Component%20Object%20Reference) (OtherBodyIndex :type Integer) (bFromSweep :type Boolean) (SweepResult :type Hit%20Result%20Structure%20%28by%20ref%29))
  (bind _target (Variables|Default|GetTarget))
  (bind _blockmatches (CallFunction|TrytoAttachBlock OverlappedComponent OtherComp (Variables|Default|GetRedBlock) (Variables|Default|GetRedBlockGrabComponent)))
  (Variables|Default|SetIsRedBlockInPlace _blockmatches)
  (bind _solved (CallFunction|CheckforSolvedPuzzle))
  (if _solved
    (Default|Turnon _target)
    (else
      (Default|TurnOff _target)
      (Development|PrintString "Turned off"))))

(event OnDropped(BlueBlockGrabComponent)
  (bind _isoverlapping (CallFunction|SetPhysicsonRelease (Variables|Default|GetBlueBlock) (Variables|Default|GetBlueCubeLocation)))
  (Variables|Default|SetIsBlueBlockInPlace _isoverlapping)
  (CallFunction|CheckforSolvedPuzzle))

(event EventBeginPlay)

(event Collision|EventActorBeginOverlap
  (params (OtherActor :type Actor%20Object%20Reference)))

(event EventTick
  (params (DeltaSeconds :type Float%20%28single-precision%29)))

(fn ConstructionScript)

(fn SetPhysicsonRelease
  (params (Block :type Primitive%20Component%20Object%20Reference) (CubeLocation :type Primitive%20Component%20Object%20Reference))
  (bind _returnvalue (Class|PrimitiveComponent|IsOverlappingComponent Block CubeLocation))
  (if _returnvalue
    (Physics|SetSimulatePhysics Block false)
    (else
      (Physics|SetSimulatePhysics Block true)))
  (return _returnvalue))

(fn TrytoAttachBlock
  (params (OverlappedLocation :type Primitive%20Component%20Object%20Reference) (OverlappingObject :type Primitive%20Component%20Object%20Reference) (CorrectBlock :type Primitive%20Component%20Object%20Reference) (CorrectGrabComponent :type Grab%20Component%20Object%20Reference))
  (bind _returnvalue (== OverlappingObject CorrectBlock))
  (if _returnvalue
    (Default|TryRelease CorrectGrabComponent)
    (Transformation|AttachComponentToComponent OverlappingObject OverlappedLocation "None" "SnapToTarget" "SnapToTarget" "KeepWorld" true))
  (return _returnvalue))

(fn CheckforSolvedPuzzle
  (bind _isredblockinplace (Variables|Default|GetIsRedBlockInPlace))
  (bind _isblueblockinplace (Variables|Default|GetIsBlueBlockInPlace))
  (bind _solvedlight (Variables|Default|GetSolvedLight))
  (bind _returnvalue (and _isredblockinplace _isblueblockinplace))
  (if _returnvalue
    (Rendering|Components|Light|SetLightColor _solvedlight "(R=0.079539,G=1.000000,B=0.000000,A=1.000000)" true)
    (else
      (Rendering|Components|Light|SetLightColor _solvedlight "(R=1.000000,G=0.000000,B=0.000000,A=1.000000)" true)))
  (return _returnvalue))
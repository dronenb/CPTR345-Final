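; BP_Doorway is a VR Labs prop door that slides open and closed when switched by its Turnon and TurnOff events.
; BeginPlay caches the door's starting world location, and a DoorOpen flag ignores repeated calls.
; A timeline plays or reverses, moving the door backward along its forward vector by a percentage of MaximumTravel from that start point.
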(event EventBeginPlay
  (Variables|Default|SetInitialLocation (Transformation|GetWorldLocation (Variables|Default|GetDoor)))
  (Components|Timeline|SetPlayRate (Variables|Default|GetDoor%20Animation) 1.0))

(event Collision|EventActorBeginOverlap
  (params (OtherActor :type Actor%20Object%20Reference)))

(event EventTick
  (params (DeltaSeconds :type Float%20%28single-precision%29)))

(event EventTurnon
  (bind _door (Variables|Default|GetDoor))
  (Development|PrintString "Opening the door!")
  (if (not (Variables|Default|GetDoorOpen))
    (Variables|Default|SetDoorOpen true)
    (bind _percent_travel (Timeline|Door%20Animation Play)
      (:Update
        (Transformation|SetWorldLocation _door (- (Variables|Default|GetInitialLocation) (* (Math|Vector|GetForwardVector _door) (* _percent_travel (Variables|Default|GetMaximum%20Travel)))) false false)))))

(event EventTurnOff
  (bind _door (Variables|Default|GetDoor))
  (if (Variables|Default|GetDoorOpen)
    (Variables|Default|SetDoorOpen false)
    (bind _percent_travel (Timeline|Door%20Animation Reverse)
      (:Update
        (Transformation|SetWorldLocation _door (- (Variables|Default|GetInitialLocation) (* (Math|Vector|GetForwardVector _door) (* _percent_travel (Variables|Default|GetMaximum%20Travel)))) false false)))))

(fn ConstructionScript)